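; A damage volume that periodically applies a Gameplay Ability System effect to characters inside its box.
; A looping half-second timer starts on BeginPlay and checks the actors overlapping the box, printing a debug string for each GASCharacterBase.
; Living characters with a valid ability system component apply the configured GameplayEffect to themselves, with Magnitude passed through the Data.Damage SetByCaller tag.
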(event `self.ReceiveBeginPlay`
  (`KismetSystemLibrary.K2_SetTimerDelegate` (delegate `Damage Tick`) 0.5 true))

(event `Damage Tick`
  (for _array_element (`PrimitiveComponent.GetOverlappingActors` (`self.Box`) null)
    (bind _asgascharacter_base (cast `GASCharacterBase` _array_element))
    (`KismetSystemLibrary.PrintString` "Hello")
    (bind _returnvalue (`AbilitySystemBlueprintLibrary.GetAbilitySystemComponent` _asgascharacter_base))
    (if (and (`GASCharacterBase.IsAlive` _asgascharacter_base) (`KismetSystemLibrary.IsValid` _returnvalue))
      (bind _returnvalue_2 (`AbilitySystemBlueprintLibrary.AssignTagSetByCallerMagnitude` (`AbilitySystemComponent.MakeOutgoingSpec` _returnvalue (`self.Gameplay Effect Class`) 1.0 (`AbilitySystemComponent.MakeEffectContext` _returnvalue)) (struct :`TagName` "Data.Damage") (`self.Magnitude`)))
      (`AbilitySystemComponent.BP_ApplyGameplayEffectSpecToSelf` _returnvalue _returnvalue_2))))

(fn `UserConstructionScript`)