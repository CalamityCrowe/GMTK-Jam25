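; BP_WaveManager continuously spawns melee and ranged enemies at locations chosen by an environment query.
; A looping timer runs the EQS_SpawnPoints query from the manager and caches all matching locations after a short delay.
; A second looping timer drives spawning, randomly choosing an enemy type and a cached point.
; Ranged spawns are raised slightly and skipped if still colliding after adjustment, while melee always spawns.
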(event `Spawn Enemy`
  (if (> (`KismetArrayLibrary.Array_Length` (`self.Spawn Locations`)) 0)
    (switch `int` (`KismetMathLibrary.RandomInteger` 2)
      (:`0`
        (`|SpawnActorFromClass` (`self.MeleeContext`) (`KismetMathLibrary.MakeTransform` (`KismetArrayLibrary.Array_Random` (`self.Spawn Locations`))) "AdjustIfPossibleButAlwaysSpawn" "MultiplyWithRoot" null null))
      (:`1`
        (`|SpawnActorFromClass` (`self.RangedContext`) (`KismetMathLibrary.MakeTransform` (+ (`KismetArrayLibrary.Array_Random` (`self.Spawn Locations`)) (0.0 0.0 50.0))) "AdjustIfPossibleButDontSpawnIfColliding" "MultiplyWithRoot" null null)))))

(event `self.ReceiveBeginPlay`
  (`KismetSystemLibrary.K2_SetTimerDelegate` (delegate `UpdateSpawnPoint`) 0.5 true)
  (`KismetSystemLibrary.K2_SetTimerDelegate` (`|CreateDelegate` :!event `Spawn Enemy`) 2.0 true))

(event `UpdateSpawnPoint`
  (bind _returnvalue (`EnvQueryManager.RunEQSQuery` "/Game/GAS/Blueprints/Wave_Manager/EQS_SpawnPoints.EQS_SpawnPoints" self "AllMatching" "/Script/AIModule.EnvQueryInstanceBlueprintWrapper"))
  (`KismetSystemLibrary.Delay` 0.2)
  (bind _resultlocations (`EnvQueryInstanceBlueprintWrapper.GetQueryResultsAsLocations` _returnvalue))
  (set `self.Spawn Locations` _resultlocations))

(fn `SpawnEnemy`
  (params (SpawnLocations :type "Array of Vector Structure")))

(fn `UserConstructionScript`)